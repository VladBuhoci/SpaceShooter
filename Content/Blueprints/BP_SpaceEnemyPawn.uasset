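; BP_SpaceEnemyPawn is a space enemy pawn that displays its name, hit points and shield points through a widget component.
; On BeginPlay it copies its name and maximum hit and shield values into the BP_NPC_HP_SP_Stats widget.
; Every Tick it pushes current hit and shield values to that widget, repeating the lookup and cast for each write rather than caching the reference.
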(event EventBeginPlay
  (bind _survivabilitysummarywidgetcomponent (Variables|Default|GetSurvivabilitySummaryWidgetComponent))
  (bind _returnvalue (UserInterface|GetUserWidgetObject _survivabilitysummarywidgetcomponent))
  (bind _asbp_npc_hp_sp_stats (Utilities|Casting|CastToBP_NPC_HP_SP_Stats _returnvalue))
  (Variables|/Game/Blueprints/UI/Widgets/BP_NPC_HP_SP_Stats.BP_NPC_HP_SP_Stats_C|SetMax%20Hit%20Points _asbp_npc_hp_sp_stats (Variables|Default|GetMaxHitPoints))
  (Variables|/Game/Blueprints/UI/Widgets/BP_NPC_HP_SP_Stats.BP_NPC_HP_SP_Stats_C|SetMax%20Shield%20Points _asbp_npc_hp_sp_stats (Variables|Default|GetMaxShieldPoints))
  (Variables|/Game/Blueprints/UI/Widgets/BP_NPC_HP_SP_Stats.BP_NPC_HP_SP_Stats_C|SetName _asbp_npc_hp_sp_stats (Variables|Default|GetName)))

(event EventTick
  (params (DeltaSeconds :type Float%20%28single-precision%29))
  (bind _survivabilitysummarywidgetcomponent (Variables|Default|GetSurvivabilitySummaryWidgetComponent))
  (bind _returnvalue (UserInterface|GetUserWidgetObject _survivabilitysummarywidgetcomponent))
  (bind _asbp_npc_hp_sp_stats (Utilities|Casting|CastToBP_NPC_HP_SP_Stats _returnvalue))
  (Variables|/Game/Blueprints/UI/Widgets/BP_NPC_HP_SP_Stats.BP_NPC_HP_SP_Stats_C|SetCurrent%20Hit%20Points _asbp_npc_hp_sp_stats (Variables|Default|GetCurrentHitPoints))
  (Variables|/Game/Blueprints/UI/Widgets/BP_NPC_HP_SP_Stats.BP_NPC_HP_SP_Stats_C|SetCurrent%20Shield%20Points _asbp_npc_hp_sp_stats (Variables|Default|GetCurrentShieldPoints)))

(fn ConstructionScript)