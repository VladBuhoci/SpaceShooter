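; Base loot chest Blueprint that drives its tooltip and contents-overview widgets.
; On begin play it sets the tooltip to the chest name and caches the overview widget, which receives the contained item boxes just before opening.
; Events for cycling and grabbing item boxes update the overview's highlight and entries.
; When the chest is emptied, the tooltip name changes to "Empty Chest".
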(event EventBeginPlay
  (bind _asbp_loot_chest_tooltip_widget (Utilities|Casting|CastToBP_LootChest_TooltipWidget (UserInterface|GetUserWidgetObject (Variables|Default|GetInfoWidgetComponent))))
  (Variables|/Game/Blueprints/UI/Widgets/BP_LootChest_TooltipWidget.BP_LootChest_TooltipWidget_C|SetName _asbp_loot_chest_tooltip_widget (Variables|Default|GetChestName))
  (bind _asbp_loot_chest_all_items_overview_widget (Utilities|Casting|CastToBP_LootChest_AllItemsOverviewWidget (UserInterface|GetUserWidgetObject (Variables|Default|GetChestOverviewWidgetComponent))))
  (Variables|Default|SetAll%20items%20Overview%20Widget _asbp_loot_chest_all_items_overview_widget))

(event EventOnChestEmptied
  (bind _asbp_loot_chest_tooltip_widget (Utilities|Casting|CastToBP_LootChest_TooltipWidget (UserInterface|GetUserWidgetObject (Variables|Default|GetInfoWidgetComponent))))
  (Variables|/Game/Blueprints/UI/Widgets/BP_LootChest_TooltipWidget.BP_LootChest_TooltipWidget_C|SetName _asbp_loot_chest_tooltip_widget "Empty Chest"))

(event EventOnHighlightPreviousItemBoxInsideChest
  (Default|HighlightItem (Variables|Default|GetAll%20items%20Overview%20Widget) (Class|LootChest|GetCurrentItemBoxIndex)))

(event EventOnHighlightNextItemBoxInsideChest
  (Default|HighlightItem (Variables|Default|GetAll%20items%20Overview%20Widget) (Class|LootChest|GetCurrentItemBoxIndex)))

(event EventOnGrabHighlightedItemBoxfromChest
  (params (RemovedHighlightedItemBoxIndex :type Integer) (bRemoveItem :type Boolean))
  (Default|RemoveHighlightedItem (Variables|Default|GetAll%20items%20Overview%20Widget) RemovedHighlightedItemBoxIndex (Class|LootChest|GetCurrentItemBoxIndex) bRemoveItem))

(event EventOnChestPreOpen
  (Default|SupplyItemsData (Variables|Default|GetAll%20items%20Overview%20Widget) (Class|LootChest|GetContainedItemBoxes)))

(fn ConstructionScript)