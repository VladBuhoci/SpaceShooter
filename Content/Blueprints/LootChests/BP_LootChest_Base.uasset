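; Base loot chest Blueprint that drives the chest's tooltip and contained-items overview widgets.
; On BeginPlay it sets the chest name on the tooltip and caches the overview widget, both taken from widget components.
; Chest events then update the overview: pre-open supplies the contained items, next/previous highlights the current index, and grabbing removes the highlighted item.
; The item list and current index come from getters defined outside this graph.
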(event EventBeginPlay
  (bind _asbp_loot_chest_tooltip_widget (Utilities|Casting|CastToBP_LootChest_TooltipWidget (UserInterface|GetUserWidgetObject (Variables|Default|GetInfoWidgetComponent))))
  (Variables|/Game/Blueprints/UI/Widgets/BP_LootChest_TooltipWidget.BP_LootChest_TooltipWidget_C|SetName _asbp_loot_chest_tooltip_widget (Variables|Default|GetChestName))
  (bind _asbp_loot_chest_all_items_overview_widget (Utilities|Casting|CastToBP_LootChest_AllItemsOverviewWidget (UserInterface|GetUserWidgetObject (Variables|Default|GetItemsOverviewWidgetComponent))))
  (Variables|Default|SetAll%20items%20Overview%20Widget _asbp_loot_chest_all_items_overview_widget))

(event EventOnChestPreOpen
  (Default|SupplyItemsData (Variables|Default|GetAll%20items%20Overview%20Widget) (Class|LootChest|GetContainedItems)))

(event EventOnHighlightPreviousItemInsideChest
  (Default|HighlightItem (Variables|Default|GetAll%20items%20Overview%20Widget) (Class|LootChest|GetCurrentItemIndex)))

(event EventOnHighlightNextItemInsideChest
  (Default|HighlightItem (Variables|Default|GetAll%20items%20Overview%20Widget) (Class|LootChest|GetCurrentItemIndex)))

(event EventOnGrabHighlightedItemfromChest
  (params (RemovedHighlightedItemIndex :type Integer))
  (Default|RemoveHighlightedItem (Variables|Default|GetAll%20items%20Overview%20Widget) RemovedHighlightedItemIndex (Class|LootChest|GetCurrentItemIndex)))

(fn ConstructionScript)