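; Development weapon Blueprint that uses a spotlight to show the weapon's current spread cone.
; The construction script snaps the SpotLight to the Muzzle socket on MeshComponent.
; Each Tick sets both inner and outer cone angles to SpreadAngle scaled down by CurrentAccuracy as a percentage, so higher accuracy narrows the hard-edged beam.
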(event EventBeginPlay)

(event Collision|EventActorBeginOverlap
  (params (OtherActor :type Actor%20Object%20Reference)))

(event EventTick
  (params (DeltaSeconds :type Float%20%28single-precision%29))
  (bind _spreadangle (Variables|Default|GetSpreadAngle))
  (bind _currentaccuracy (Variables|Default|GetCurrentAccuracy))
  (bind _returnvalue (* 2 _spreadangle))
  (bind _returnvalue_2 (/ _currentaccuracy 1e+02))
  (bind _returnvalue_3 (* _returnvalue _returnvalue_2))
  (bind _returnvalue_4 (- _returnvalue _returnvalue_3))
  (bind _returnvalue_5 (/ _returnvalue_4 2.0))
  (Rendering|Lighting|SetOuterConeAngle (Variables|Default|GetSpotLight) _returnvalue_5)
  (Rendering|Lighting|SetInnerConeAngle (Variables|Default|GetSpotLight) _returnvalue_5))

(fn ConstructionScript
  (Transformation|AttachComponentToComponent (Variables|Default|GetSpotLight) (Variables|Default|GetMeshComponent) "Muzzle" "SnapToTarget" "SnapToTarget" "SnapToTarget" true))