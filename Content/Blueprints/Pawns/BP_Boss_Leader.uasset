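; Boss leader pawn for a space shooter whose destruction wipes out the remaining enemies.
; On BeginPlay it binds to its own OnDestroyed event, which calls DestroyRemainingEnemies.
; That function gathers every SpaceEnemyPawn in the level and applies overkill damage to those not yet destroyed, so they die through the damage path rather than a direct destroy.
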(event Custom|OnBossDestroyed
  (params (DestroyedActor :type Actor%20Object%20Reference))
  (Utilities|DestroyRemainingEnemies))

(event EventBeginPlay
  (|CallParentFunction)
  (EventDispatchers|BindEventtoOnDestroyed (delegate Custom|OnBossDestroyed)))

(event EventTick
  (params (DeltaSeconds :type Float%20%28single-precision%29))
  (|CallParentFunction 0.0))

(fn ConstructionScript)