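; Player spacecraft pawn that uses a spotlight to visualize the equipped weapon's current aim spread.
; The construction script snaps the SpotLight to a weapon attach socket on the spacecraft mesh.
; Every tick, both inner and outer cone angles are set to the weapon's spread angle scaled down by its current accuracy, so the beam narrows as accuracy rises.
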(event EventBeginPlay)

(event Collision|EventActorBeginOverlap
  (params (OtherActor :type Actor%20Object%20Reference)))

(event EventTick
  (params (DeltaSeconds :type Float%20%28single-precision%29))
  (bind _equippedweapon (Variables|Default|GetEquippedWeapon))
  (bind _weaponattributes (Variables|/Script/SpaceShooter.Weapon|GetWeaponAttributes _equippedweapon))
  (bind _currentaccuracy (Variables|/Script/SpaceShooter.Weapon|GetCurrentAccuracy _equippedweapon))
  (bind _spreadangle (Utilities|Struct|BreakWeaponAttributes _weaponattributes))
  (bind _returnvalue (/ _currentaccuracy 1e+02))
  (bind _returnvalue_2 (* 2 _spreadangle))
  (bind _returnvalue_3 (* _returnvalue_2 _returnvalue))
  (bind _returnvalue_4 (- _returnvalue_2 _returnvalue_3))
  (bind _returnvalue_5 (/ _returnvalue_4 2.0))
  (Rendering|Lighting|SetOuterConeAngle (Variables|Default|GetSpotLight) _returnvalue_5)
  (Rendering|Lighting|SetInnerConeAngle (Variables|Default|GetSpotLight) _returnvalue_5))

(fn ConstructionScript
  (Transformation|AttachComponentToComponent (Variables|Default|GetSpotLight) (Variables|Default|GetSpacecraftMeshComponent) "Weapon_AttachPoint_DEV" "SnapToTarget" "SnapToTarget" "SnapToTarget" true))