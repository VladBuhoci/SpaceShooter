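; Space game instance that builds the campaign's missions and chapters when the game initializes.
; Init registers a "Training" mission with three "Newbie Ground" chapters, plus an "Advanced Training" mission with no chapters.
; Each chapter pairs a level with a destroy-everyone goal that spawns a growing number of BP_SpaceEnemyPawn enemies and uses the genocide goal widget.
; Chapters are added in a chain, each call feeding its result into the next.
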(event EventInit
  (Utilities|FlowControl|Sequence
    (:then_0
      (bind _createdmission (Class|SpaceGameInstance|AddCampaignMission "/Script/SpaceShooter.CampaignMissionDescription" "Training"))
      (bind _genocidegoal (Class|SpaceGameInstance|CreateGoalOfTypeDestroyEveryone (Utilities|Struct|MakeNpcSpawnRules (Utilities|Array|MakeArray (Utilities|Struct|MakeSpawnableNPC "/Game/Blueprints/BP_SpaceEnemyPawn.BP_SpaceEnemyPawn_C" 1e+02)) 2 2e+03 1e+03 2 2 8.0 12.0) "/Game/Blueprints/UI/Widgets/BP_CampaignMode_GenocideGoalWidget.BP_CampaignMode_GenocideGoalWidget_C"))
      (bind _campaignmission (Class|SpaceGameInstance|AddCampaignChapter "/Script/SpaceShooter.CampaignChapterDescription" "Newbie Ground" "Level01" _genocidegoal _createdmission))
      (bind _genocidegoal_2 (Class|SpaceGameInstance|CreateGoalOfTypeDestroyEveryone (Utilities|Struct|MakeNpcSpawnRules (Utilities|Array|MakeArray (Utilities|Struct|MakeSpawnableNPC "/Game/Blueprints/BP_SpaceEnemyPawn.BP_SpaceEnemyPawn_C" 1e+02)) 3 2e+03 1e+03 3 4 7.0 9.0) "/Game/Blueprints/UI/Widgets/BP_CampaignMode_GenocideGoalWidget.BP_CampaignMode_GenocideGoalWidget_C"))
      (bind _campaignmission_2 (Class|SpaceGameInstance|AddCampaignChapter "/Script/SpaceShooter.CampaignChapterDescription" "Newbie Ground 2" "00_Dev_ExperimentalSpace" _genocidegoal_2 _campaignmission))
      (bind _genocidegoal_3 (Class|SpaceGameInstance|CreateGoalOfTypeDestroyEveryone (Utilities|Struct|MakeNpcSpawnRules (Utilities|Array|MakeArray (Utilities|Struct|MakeSpawnableNPC "/Game/Blueprints/BP_SpaceEnemyPawn.BP_SpaceEnemyPawn_C" 1e+02)) 5 2e+03 1e+03 3 4 7.0 9.0) "/Game/Blueprints/UI/Widgets/BP_CampaignMode_GenocideGoalWidget.BP_CampaignMode_GenocideGoalWidget_C"))
      (Class|SpaceGameInstance|AddCampaignChapter "/Script/SpaceShooter.CampaignChapterDescription" "Newbie Ground 3" "00_Dev_ExperimentalSpace" _genocidegoal_3 _campaignmission_2))
    (:then_1
      (Class|SpaceGameInstance|AddCampaignMission "/Script/SpaceShooter.CampaignMissionDescription" "Advanced Training"))))